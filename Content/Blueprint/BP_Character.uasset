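; BP_Character is a character Blueprint that puts the WBP_GameScreen HUD widget on the viewport at BeginPlay.
; The IA_ToggleUI input event is empty, and the FlipFlop meant to show and remove WBP_MagicCustomize, toggling cursor and look-input ignore, is disconnected.
; The assignments storing both widgets in MainScreen and CustomMagicUI are also unwired, so neither reference is saved.
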(event Input|EnhancedActionEvents|EnhancedInputActionIA_ToggleUI
  (params (ActionValue :type Boolean) (ElapsedSeconds :type Float%20%28double-precision%29) (TriggeredSeconds :type Float%20%28double-precision%29) (InputAction :type Input%20Action%20Object%20Reference :default "/Game/Core/Input/IA_ToggleUI.IA_ToggleUI")))

(event EventBeginPlay
  (bind _returnvalue (UserInterface|CreateWidget "/Game/Blueprint/WBP_GameScreen.WBP_GameScreen_C"))
  (UserInterface|Viewport|AddtoViewport _returnvalue 0))

(event Collision|EventActorBeginOverlap
  (params (OtherActor :type Actor%20Object%20Reference)))

(event EventTick
  (params (DeltaSeconds :type Float%20%28single-precision%29)))

(fn ConstructionScript)